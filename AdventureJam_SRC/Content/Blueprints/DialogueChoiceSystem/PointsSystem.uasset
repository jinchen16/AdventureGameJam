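; PointsSystem is an actor in the dialogue choice system that keeps a running points total.
; The AddPoints event adds the given amount to PointsAccum.
; Its construction script enforces a single instance: if more than one PointsSystem exists, it stores the first one found in Instance, prints that it already exists and destroys itself.
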(event Custom|AddPoints
  (params (Amount :type Integer))
  (Variables|Default|SetPointsAccum (+ (Variables|Default|GetPointsAccum) Amount)))

(event EventBeginPlay)

(event Collision|EventActorBeginOverlap
  (params (OtherActor :type Actor%20Object%20Reference)))

(event EventTick
  (params (DeltaSeconds :type Float%20%28single-precision%29)))

(fn ConstructionScript
  (bind _outactors (Actor|GetAllActorsOfClass "PointsSystem_C"))
  (if (> (Utilities|Array|Length _outactors) 1)
    (bind _output_get (Variables|Default|SetInstance (Utilities|Array|Get(acopy) _outactors)))
    (Development|PrintString (Utilities|String|Append (Utilities|GetDisplayName _output_get) "already exists"))
    (Actor|DestroyActor)))