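; ChoiceSystemHandler is a Blueprint that runs dialogue choice events and accumulates points.
; On BeginPlay it loads every Events data table row into an array, from which a choice is selected by index.
; It builds a ChoiceUI widget from the selected header and options, passing itself and a scene template reference to each button creation call.
; Separate events add points to the running total and remove the widget.
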(event Custom|AddPoints
  (params (Amount :type Integer))
  ;[1 1 1] Add Points to the Accumulation
  (Variables|Default|SetPointsAccum (+ (Variables|Default|GetPointsAccum) Amount)))

(event Custom|AccessEventByIndex
  (params (Index :type Integer))
  ;[1 1 1] Acces Event By Index - Get one element form the choices array by the index position
  (Variables|Default|SetChoice (Utilities|Array|Get(acopy) (Variables|Default|GetChoicesArray) Index)))

(event Custom|LoadChoice
  ;[1 1 1] Load Choice - Load the data to fill the array of events
  (bind _outrownames (DataTable|GetDataTableRowNames "/Game/Blueprints/DialogueChoiceSystem/events.events"))
  (for _array_element _outrownames
    (bind _returnvalue (Utilities|GetDataTableRow "/Game/Blueprints/DialogueChoiceSystem/events.events" _array_element)
      (:then
        (Utilities|Array|Add (Variables|Default|GetChoicesArray) _returnvalue)))))

(event Custom|ShowChoiceUI
  (bind _choice (Variables|Default|GetChoice))
  (bind (_name _eventid _eventheader _options) (Utilities|Struct|BreakVN_EventStruct _choice))
  ;[1 1 1] Show Choice UI - Setting header and options buttons
  (bind _returnvalue (UserInterface|CreateWidget "/Game/Blueprints/DialogueChoiceSystem/ChoiceUI.ChoiceUI_C"))
  (bind _output_get (Variables|Default|SetchoiceUI _returnvalue))
  (UserInterface|Viewport|AddtoViewport _output_get 0)
  (Default|SetHeaderText (Variables|Default|GetchoiceUI) _eventheader)
  (for _array_element _options
    (Default|CreateButtons (Variables|Default|GetchoiceUI) _array_element (Variables|Default|GetPointSystemInstance) (Variables|Default|GetSceneTemplateInstance))))

(event Custom|EndChoice
  ;[1 1 1] Close Choice Widget
  (Widget|RemovefromParent (Variables|Default|GetchoiceUI)))

(event EventBeginPlay
  (Variables|Default|SetPointSystemInstance self)
  (Development|PrintString "This is the beginning of me!")
  (CallFunction|LoadChoice))

(fn ConstructionScript)