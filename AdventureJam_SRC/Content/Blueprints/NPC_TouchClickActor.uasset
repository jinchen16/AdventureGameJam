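; Clickable NPC actor that starts a dialogue scene, gated by how many characters the player has spoken to.
; On click it picks not-enough, new or done text, incrementing the PlayerPawn's CharactersSpokenTo on the first successful conversation.
; It teleports the player to ToLocation and spawns SceneTemplate with itself and the chosen text.
; GoHome returns the player to FromLocation; ScenePlaying blocks re-clicks and is not cleared here.
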(event Custom|GoHome
  (Transformation|SetActorLocation (Game|Player|GetPlayerPawn 0) (Transformation|GetActorLocation (Variables|Default|GetFromLocation)) false false))

(event MouseInput|EventActorOnClicked
  (params (ButtonPressed :type Key%20Structure :default "None"))
  (if (not (Variables|Default|GetScenePlaying))
    (bind _outactors (Actor|GetAllActorsOfClass "/Game/Blueprints/PlayerPawn.PlayerPawn_C"))
    (bind _asplayer_pawn (Utilities|Casting|CastToPlayerPawn (Utilities|Array|Get(acopy) _outactors)))
    (if (>= (Variables|/Game/Blueprints/PlayerPawn.PlayerPawn_C|GetCharactersSpokenTo _asplayer_pawn) (Variables|Default|GetMinCharactersSpokenTo))
      (if (Variables|Default|GetScenePlayed)
        (Variables|Default|SetDialogueText (Variables|Default|GetDoneText))
        (else
          (bind _outactors_2 (Actor|GetAllActorsOfClass "/Game/Blueprints/PlayerPawn.PlayerPawn_C"))
          (Variables|/Game/Blueprints/PlayerPawn.PlayerPawn_C|SetCharactersSpokenTo (Utilities|Array|Get(acopy) _outactors_2) (+ (Variables|/Game/Blueprints/PlayerPawn.PlayerPawn_C|GetCharactersSpokenTo _asplayer_pawn) 1))
          (Variables|Default|SetDialogueText (Variables|Default|GetNewText))
          (Variables|Default|SetScenePlayed true)))
      (else
        (Variables|Default|SetDialogueText (Variables|Default|GetNotEnoughText))))
    (Transformation|SetActorLocation (Game|Player|GetPlayerPawn 0) (Transformation|GetActorLocation (Variables|Default|GetToLocation)) false false)
    (Variables|Default|SetScenePlaying true)
    (bind _returnvalue (Game|SpawnActorfromClass "/Game/Blueprints/SceneTemplate.SceneTemplate_C" (Transformation|GetActorTransform) "Undefined" 0 0))
    (bind _output_get (Variables|Default|SetCurrentScene _returnvalue))
    (Variables|/Game/Blueprints/SceneTemplate.SceneTemplate_C|SetSceneStartActor _output_get self)
    (Default|InitiateNewScene _output_get (Variables|Default|GetDialogueText))))

(fn ConstructionScript)