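; SceneTemplate is an actor that plays a dialogue scene line by line from a data table.
; InitiateNewScene caches the rows and creates a DisplayDialogue widget, which PlayLine fills with speaker and text.
; NextLine input advances after a short lockout; event-flagged rows hide the dialogue and open the ChoiceSystemHandler's choice UI by EventID.
; After the last row, it removes the widget, destroys itself and tells SceneStartActor to GoHome.
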(event Custom|InitiateNewScene
  (params (CurrentScene :type Data%20Table%20Object%20Reference))
  ;[1 1 1] Initiate the scene
  (bind _outrownames (DataTable|GetDataTableRowNames CurrentScene))
  (for _array_element _outrownames
    (bind _returnvalue (Utilities|GetDataTableRow CurrentScene _array_element)
      (:then
        (Utilities|Array|Add (Variables|Default|GetArrayOfRows) _returnvalue))))
  (bind _returnvalue_2 (UserInterface|CreateWidget "/Game/Blueprints/DisplayDialogue.DisplayDialogue_C"))
  (bind _output_get (Variables|Default|SetDisplayDialogueWidget _returnvalue_2))
  (UserInterface|Viewport|AddtoViewport _output_get 0)
  (CallFunction|PlayLine))

(event Custom|PlayLine
  (bind _arrayofrows (Variables|Default|GetArrayOfRows))
  (bind _displaydialoguewidget (Variables|Default|GetDisplayDialogueWidget))
  (bind _row (Variables|Default|GetRow))
  (bind _output (Utilities|Array|Get(acopy) _arrayofrows _row))
  (bind (_speaker _text _event _eventid) (Utilities|Struct|BreakVN_SceneStruct _output))
  ;[1 1 1] Display a line
  (Variables|Default|SetRowFinished false)
  (if (>= (Variables|Default|GetRow) (Utilities|Array|Length (Variables|Default|GetArrayOfRows)))
    (CallFunction|EndScene)
    (else
      (Utilities|IsValid _displaydialoguewidget
        (:Is%20Valid
          (Variables|Default|SetIsEvent _event)
          (Variables|Default|SetEventID _eventid)
          (Variables|/Game/Blueprints/DisplayDialogue.DisplayDialogue_C|SetSpeaker _displaydialoguewidget (Utilities|Text|ToText(String) (Utilities|String|EnumtoString _speaker)))
          (Variables|/Game/Blueprints/DisplayDialogue.DisplayDialogue_C|SetText _displaydialoguewidget (Utilities|Text|ToText(String) _text))
          (Utilities|FlowControl|Delay 0.2)
          (Variables|Default|SetRowFinished true))))))

(event Custom|EndScene
  ;[1 1 1] End scene and kill everything
  (Widget|RemovefromParent (Variables|Default|GetDisplayDialogueWidget))
  (Variables|/Game/Blueprints/NPC_TouchClickActor.NPC_TouchClickActor_C|SetScenePlaying (Variables|Default|GetSceneStartActor) false)
  (Actor|DestroyActor)
  (Default|GoHome (Variables|Default|GetSceneStartActor)))

(event EventBeginPlay
  ;[1 1 1] SceneTemplate Initialization
  ;;[1 1 1] Allow player input
  (Input|EnableInput (Game|GetPlayerController 0))
  (bind _outactors (Actor|GetAllActorsOfClass "/Game/Blueprints/DialogueChoiceSystem/ChoiceSystemHandler.ChoiceSystemHandler_C"))
  (Utilities|IsValid (Utilities|Array|Get(acopy) _outactors)
    (:Is%20Valid
      (bind _output_get (Variables|Default|SetChoiceSystemHandler (Utilities|Array|Get(acopy) _outactors)))
      (Variables|/Game/Blueprints/DialogueChoiceSystem/ChoiceSystemHandler.ChoiceSystemHandler_C|SetSceneTemplateInstance _output_get self))))

(event Input|ActionEvents|InputActionNextLine
  (params (Key :type Key%20Structure :default "None"))
  (bind _choicesystemhandler (Variables|Default|GetChoiceSystemHandler))
  ;[1 1 1] Go to the next line based on input
  (:Pressed
    (if (Variables|Default|GetRowFinished)
      (Variables|Default|SetRow (+ (Variables|Default|GetRow) 1))
      (if (Variables|Default|GetIsEvent)
        (Default|AccessEventbyIndex _choicesystemhandler (Variables|Default|GetEventID))
        (Default|ShowChoiceUI _choicesystemhandler)
        (Widget|SetVisibility (Variables|Default|GetDisplayDialogueWidget) "Hidden")
        (else
          (CallFunction|PlayLine))))))

(fn ConstructionScript)